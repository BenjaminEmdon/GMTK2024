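; BP_LocationVolume is a trigger volume that records which grid column or row the player character has entered.
; When BP_PlayerCharacter begins overlapping its Box, SetPlayerLocation writes either the column letter or the row number into the player's Location, according to GridLineType.
; Each volume updates one axis and preserves the other, so column and row volumes together form the full grid coordinate.
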(event `self.ReceiveBeginPlay`)

(event `self.Box.OnComponentBeginOverlap`
  (params (OverlappedComponent :type "PrimitiveComponent Object Reference") (OtherActor :type "Actor Object Reference") (OtherComp :type "PrimitiveComponent Object Reference") (OtherBodyIndex :type Integer) (bFromSweep :type Boolean) (SweepResult :type "HitResult Structure (by ref)"))
  (bind _asbp_player_character (cast `/Game/Scripts/BP_PlayerCharacter` OtherActor))
  (`self.SetPlayerLocation` _asbp_player_character))

(fn `SetPlayerLocation`
  (params (PlayerRef :type "/Game/Scripts/BP_PlayerCharacter Object Reference"))
  (bind _location_column (break `/Game/Scripts/Structs/FLocation` (`/Game/Scripts/BP_PlayerCharacter.Location` PlayerRef)))
  (bind (_location_column_2 _location_row) (break `/Game/Scripts/Structs/FLocation` (`/Game/Scripts/BP_PlayerCharacter.Location` PlayerRef)))
  (switch `/Game/Scripts/Enums/EGridDirection` (`self.GridLineType`)
    (:`NewEnumerator0`
      (set `/Game/Scripts/BP_PlayerCharacter.Location` (make `/Game/Scripts/Structs/FLocation` (`self.ColumnLetter`) _location_row) PlayerRef)
      (return))
    (:`NewEnumerator1`
      (set `/Game/Scripts/BP_PlayerCharacter.Location` (make `/Game/Scripts/Structs/FLocation` _location_column (`self.RowNumber`)) PlayerRef)
      (return))))

(fn `UserConstructionScript`)