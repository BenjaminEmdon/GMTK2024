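; BP_PlayerCharacter is the player-controlled character, handling startup registration and Enhanced Input movement.
; On BeginPlay it registers itself with BP_GameMode_Default, switches the player controller's view to the game mode's camera, and adds the default input mapping context.
; IA_Move drives movement input along forward and right vectors derived from control rotation, with pitch ignored.
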(event `self.ReceiveBeginPlay`
  (bind _returnvalue (pcsubsystem `EnhancedInputLocalPlayerSubsystem` (`self.PlayerControllerRef`)))
  (bind _asbp_game_mode_default (cast `/Game/Scripts/BP_GameMode_Default` (`GameplayStatics.GetGameMode`)))
  (set `self.GameModeRef` _asbp_game_mode_default)
  (set `/Game/Scripts/BP_GameMode_Default.Player` self (`self.GameModeRef`))
  (bind _asbp_player_controller_default (cast `/Game/Scripts/BP_PlayerController_Default` (`self.GetController`)))
  (bind _output_get (set `self.PlayerControllerRef` _asbp_player_controller_default))
  (`PlayerController.SetViewTargetWithBlend` _output_get (`/Game/Scripts/BP_GameMode_Default.Camera` (`self.GameModeRef`)) 0.0 "VTBlend_Linear" 0.0 true)
  (`/Engine/EditorBlueprintResources/StandardMacros.IsValid` _returnvalue
    (:`Is Valid`
      (`EnhancedInputSubsystemInterface.AddMappingContext` _returnvalue "/Game/Scripts/Input/IC_Default.IC_Default" 0 (struct)))))

(event `EnhancedInput|/Game/Scripts/Input/IA_Move`
  (params (ActionValue :type "Vector2D Structure") (ElapsedSeconds :type "Float (double-precision)") (TriggeredSeconds :type "Float (double-precision)") (InputAction :type "InputAction Object Reference" :default "/Game/Scripts/Input/IA_Move.IA_Move"))
  (bind (_returnvalue_roll _returnvalue_pitch _returnvalue_yaw) (`KismetMathLibrary.BreakRotator` (`self.GetControlRotation`)))
  (bind (_returnvalue_roll_2 _returnvalue_pitch_2 _returnvalue_yaw_2) (`KismetMathLibrary.BreakRotator` (`self.GetControlRotation`)))
  (:`Triggered`
    (`self.AddMovementInput` (`KismetMathLibrary.GetRightVector` (`KismetMathLibrary.MakeRotator` _returnvalue_roll 0.0 _returnvalue_yaw)) ActionValue_X)
    (`self.AddMovementInput` (`KismetMathLibrary.GetForwardVector` (`KismetMathLibrary.MakeRotator` 0.0 0.0 _returnvalue_yaw_2)) ActionValue_Y)))

(fn `UserConstructionScript`)